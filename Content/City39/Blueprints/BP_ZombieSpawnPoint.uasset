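; BP_ZombieSpawnPoint is a spawn point that periodically spawns replicated prototype zombies at its own transform.
; On BeginPlay, only the authority starts a looping timer that calls SpawnZombie.
; SpawnZombie spawns one zombie when CurrentZombieCount is below MaxZombiesAllowed, then always spawns another, so the cap does not bound spawning.
; The count update is disconnected and would count spawn points rather than zombies.
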(event EventBeginPlay
  (Networking|SwitchHasAuthority
    (:Authority
      (Utilities|Time|SetTimerbyFunctionName 0 "SpawnZombie" 5.0 true))))

(fn ConstructionScript)

(fn SpawnZombie
  (Utilities|FlowControl|Sequence
    (:then_0
      (bind _outactors (Actor|GetAllActorsOfClass "BP_ZombieSpawnPoint_C")))
    (:then_1
      (Math|Integer|CompareInt (Variables|Default|GetCurrentZombieCount) (Variables|Default|GetMaxZombiesAllowed)
        (:<
          (Game|SpawnActorfromClass "/Game/FPS_Game/Blueprints/Bonus/Replication/Interactive/Replicated_SimplePrototypingZombie.Replicated_SimplePrototypingZombie_C" (Transformation|GetActorTransform) "Undefined" 0 0))))
    (:then_2
      (Game|SpawnActorfromClass "/Game/FPS_Game/Blueprints/Bonus/Replication/Interactive/Replicated_SimplePrototypingZombie.Replicated_SimplePrototypingZombie_C" (Transformation|GetActorTransform) "Undefined" 0 0))))