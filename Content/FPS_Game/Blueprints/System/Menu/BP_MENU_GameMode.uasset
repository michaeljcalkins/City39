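; BP_MENU_GameMode is the game mode for the main menu.
; On BeginPlay it casts to BP_GameInstance and loads saved settings.
; It applies the stored resolution and fullscreen or windowed mode through an r.SetRes console command, then creates the W_MainMenu widget and adds it to the viewport.
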(event EventBeginPlay
  (bind _asbp_game_instance (Utilities|Casting|CastToBP_GameInstance (Game|GetGameInstance)))
  (bind _output_get (Variables|Default|SetGameInstanceCast _asbp_game_instance))
  (Default|LoadSettings _output_get)
  (Development|ExecuteConsoleCommand (Utilities|String|Append "r.SetRes " (Variables|/Game/FPS_Game/Blueprints/GameInstanceSettings/BP_GameInstance.BP_GameInstance_C|GetSettings_Resolution _output_get) (select (Variables|/Game/FPS_Game/Blueprints/GameInstanceSettings/BP_GameInstance.BP_GameInstance_C|GetSettings_Resolution_Mode _output_get) "f" "w")) 0)
  (bind _returnvalue (UserInterface|CreateWidget "/Game/FPS_Game/UI/W_MainMenu.W_MainMenu_C"))
  (UserInterface|Viewport|AddtoViewport _returnvalue 0))

(fn ConstructionScript)