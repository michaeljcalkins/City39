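; BP_Door is a buyable, lockable door that swings open and shut.
; Toggle events flip the open and locked states, setting the Door component's relative rotation instantly, with BeginPlay applying the initial state.
; Locking forces the door closed, and a locked door refuses to open.
; Buying assigns PlayerOwner only if none is valid, but the open and lock events never check ownership.
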(event Custom|OnOpenCloseDoor
  ;[1 1 1] Open/Close Door
  (if (Variables|Default|GetIsOpen)
    (CallFunction|CloseDoor)
    (Variables|Default|SetIsOpen false)
    (elif (not (Variables|Default|GetIsLocked))
      (CallFunction|OpenDoor)
      (Variables|Default|SetIsOpen true))))

(event Custom|OnLockUnlockDoor
  ;[1 1 1] Lock/Unlock Door
  (if (Variables|Default|GetIsLocked)
    (Variables|Default|SetIsLocked false)
    (else
      (Variables|Default|SetIsLocked true)
      (CallFunction|CloseDoor)
      (Variables|Default|SetIsOpen false))))

(event Custom|OnBuyDoor
  (params (Player :type Actor%20Object%20Reference))
  (Utilities|IsValid (Variables|Default|GetPlayerOwner)
    (:Is%20Not%20Valid
      (CallFunction|SetPlayerOwner Player))))

(event EventBeginPlay
  (if (Variables|Default|GetIsOpen)
    (CallFunction|OpenDoor)
    (else
      (CallFunction|CloseDoor))))

(fn ConstructionScript)

(fn OpenDoor
  (Transformation|SetRelativeRotation (Variables|Default|GetDoor) "0,-90.000000, 0" false false))

(fn CloseDoor
  (Transformation|SetRelativeRotation (Variables|Default|GetDoor) "0, 0, 0" false false))

(fn LockDoor
  (Variables|Default|SetIsLocked true))

(fn UnlockDoor
  (Variables|Default|SetIsLocked false))

(fn SetPlayerOwner
  (params (Player :type Actor%20Object%20Reference))
  (Variables|Default|SetPlayerOwner Player))

(fn ClearPlayerOwner
  (Variables|Default|SetPlayerOwner 0))